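; Lantern spline actor in the Lamppost assets that lays a chosen mesh and material along an editable, optionally closed spline.
; Its construction script divides the spline length by Spacing and adds three spline mesh components per step.
; Only the first of each three is shaped, using world-space locations and scaled directions; the other two are never positioned.
; An unused per-spline-point loop remains unconnected, and the event graph is empty.
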(event EventBeginPlay)

(event Collision|EventActorBeginOverlap
  (params (OtherActor :type Actor%20Object%20Reference)))

(event EventTick
  (params (DeltaSeconds :type Float%20%28single-precision%29)))

(fn ConstructionScript
  (bind _tangentscale (Variables|Default|GetTangentScale))
  (bind _spacing (Variables|Default|GetSpacing))
  (bind _spline (Variables|Default|GetSpline))
  (Spline|SetClosedLoop (Variables|Default|GetSpline) (Variables|Default|GetClosedLoop) true)
  (for _index (range 0 (.ReturnValue (Math|Float|Division(WholeandRemainder) (Spline|GetSplineLength (Variables|Default|GetSpline)) _spacing)))
    (bind _returnvalue (AddComponent|AddSplineMeshComponent true))
    (Components|StaticMesh|SetStaticMesh _returnvalue (Variables|Default|GetMesh))
    (Rendering|Material|SetMaterial _returnvalue 0 (Variables|Default|GetMaterial))
    (bind _returnvalue_2 (AddComponent|AddSplineMeshComponent true))
    (Components|StaticMesh|SetStaticMesh _returnvalue_2 (Variables|Default|GetMesh))
    (Rendering|Material|SetMaterial _returnvalue_2 0 (Variables|Default|GetMaterial))
    (bind _returnvalue_3 (AddComponent|AddSplineMeshComponent true))
    (Components|StaticMesh|SetStaticMesh _returnvalue_3 (Variables|Default|GetMesh))
    (Rendering|Material|SetMaterial _returnvalue_3 0 (Variables|Default|GetMaterial))
    (SplineMesh|SetStartandEnd _returnvalue (Spline|GetLocationatDistanceAlongSpline _spline (* _index _spacing) "World") (* (Spline|GetDirectionatDistanceAlongSpline _spline (* _index _spacing) "World") _tangentscale) (Spline|GetLocationatDistanceAlongSpline _spline (+ (* _index _spacing) _spacing) "World") (* (Spline|GetDirectionatDistanceAlongSpline _spline (+ (* _index _spacing) _spacing) "World") _tangentscale) true :!class /Script/Engine.SplineMeshComponent)))