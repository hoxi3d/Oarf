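; BP_Griffon is a quest-giver NPC that offers the first main quest when the player interacts with it.
; Tick spins its quest sign, while BeginPlay fills the interaction widget's name and makes player character 0 its owner.
; Player radius events show or hide that widget.
; Interaction adds and starts BP_Quest_Main_01 through the character's quest manager unless already present, with debug prints marking these events.
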(event EventBeginPlay
  ;[1 1 1] BeginPlay
  (bind _asw_interaction (Utilities|Casting|CastToW_Interaction (UserInterface|GetUserWidgetObject (Variables|Default|GetInteractionWidget))))
  (Rendering|Components|TextRender|SetText (Variables|/Game/HUD/Quests/NPCs/W_Interaction.W_Interaction_C|GetName _asw_interaction) (Variables|Default|GetName))
  (Actor|SetOwner (Game|GetPlayerCharacter 0)))

(event EventTick
  (params (DeltaSeconds :type Float%20%28single-precision%29))
  (Transformation|AddLocalRotation (Variables|Default|GetQuestSign) (Math|Rotator|MakeRotator 0.0 0.0 (* DeltaSeconds 4e+01)) false false))

(event EventOnEnterPlayerRadius
  (params (Character :type BP%20Oarf%20Object%20Reference))
  ;[1 1 1] RadiusVisibility
  (Rendering|SetVisibility (Variables|Default|GetInteractionWidget) true false)
  (Development|PrintString "Visible"))

(event EventOnLeavePlayerRadius
  (params (Character :type BP%20Oarf%20Object%20Reference))
  ;[1 1 1] RadiusVisibility
  (Rendering|SetVisibility (Variables|Default|GetInteractionWidget) false false)
  (Development|PrintString "Invisible"))

(event EventOnInteractwith
  (params (Character :type BP%20Oarf%20Object%20Reference))
  (bind _questmanagerref (Variables|/Game/MainAssets/Characters/MainCharacter/BPs/Blueprints/BP_Oarf.BP_Oarf_C|GetQuestManagerRef Character))
  ;[1 1 1] Interact
  (if (not (Utilities|Array|ContainsItem (Variables|/Game/MainAssets/Blueprints/Actors/BP_QuestManager.BP_QuestManager_C|GetAllQuestClasses _questmanagerref) "/Game/MainAssets/Blueprints/Actors/QuestActors/BP_Quest_Main_01.BP_Quest_Main_01_C"))
    (Default|AddNewQuest _questmanagerref "/Game/MainAssets/Blueprints/Actors/QuestActors/BP_Quest_Main_01.BP_Quest_Main_01_C" true)
    (Development|PrintString "QuestStart")))

(fn ConstructionScript)