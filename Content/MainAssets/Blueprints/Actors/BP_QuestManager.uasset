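; BP_QuestManager spawns and tracks quest actors, handles selection of the current quest and feeds goal guidance to the main widget.
; Adding a quest rejects duplicate classes, creates its list entry and selects it if requested or first.
; Switching sub-quests replaces a spawned goal actor marking the location, if any.
; Player movement updates the horizontal distance text and rotates the minimap arrow, using paired DoOnce gates to toggle visibility around a distance threshold.
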(event Custom|OnSwitchSubQuest
  (bind _currentquest (Variables|Default|GetCurrentQuest))
  (bind _mainwidget (Variables|Default|GetMainWidget))
  (Utilities|IsValid (Variables|Default|GetCurrentGoalActor)
    (:Is%20Valid
      (Actor|DestroyActor (Variables|Default|GetCurrentGoalActor)))
    (:Is%20Not%20Valid
      _))
  (bind _output_get (Variables|Default|SetCurrentSubGoal (Utilities|Array|Get(acopy) (.SubGoals (Utilities|Struct|BreakStruct_QuestInfo (Variables|/Game/MainAssets/Blueprints/Actors/QuestActors/BP_MasterQuest.BP_MasterQuest_C|GetQuestInfo _currentquest))) (Variables|/Game/MainAssets/Blueprints/Actors/QuestActors/BP_MasterQuest.BP_MasterQuest_C|GetSelectedSubGoalIndex _currentquest))))
  (if (.HasLocation (Utilities|Struct|BreakStruct_GoalLocation (.GoalLocation (Utilities|Struct|BreakStruct_GoalInfo _output_get))))
    (bind _returnvalue (Game|SpawnActorfromClass "/Game/MainAssets/Blueprints/Actors/BP_GoalActor.BP_GoalActor_C" (Math|Transform|MakeTransform (.Location (Utilities|Struct|BreakStruct_GoalLocation (.GoalLocation (Utilities|Struct|BreakStruct_GoalInfo _output_get)))) "0, 0, 0" "1,1,1") "AlwaysSpawn" 0 0))
    (Variables|Default|SetCurrentGoalActor _returnvalue)
    (bind _output_get_2 (Variables|Default|SetCurrentDistance (CallFunction|DistancetoGoal)))
    (Rendering|Components|TextRender|SetText (Variables|/Game/HUD/W_HUD.W_HUD_C|GetDistanceText (Variables|Default|GetMainWidget)) (Utilities|Text|ToText(Integer) _output_get_2 false false))
    (CallFunction|UpdateDirectionArrow)
    (Widget|SetVisibility (Variables|/Game/HUD/W_HUD.W_HUD_C|GetDistanceBorder _mainwidget) "HitTestInvisible")
    (Widget|SetVisibility (Variables|/Game/HUD/W_MiniMap.W_MiniMap_C|GetDirectionArrow (Variables|/Game/HUD/W_HUD.W_HUD_C|GetW_MiniMap _mainwidget)) (select (> (Variables|Default|GetCurrentDistance) (Variables|Default|GetShowDirectionArrowAmount)) "HitTestInvisible" "Visible"))
    (else
      (Variables|Default|SetCurrentGoalActor 0)
      (Widget|SetVisibility (Variables|/Game/HUD/W_MiniMap.W_MiniMap_C|GetDirectionArrow (Variables|/Game/HUD/W_HUD.W_HUD_C|GetW_MiniMap (Variables|Default|GetMainWidget))) "Hidden"))))

(event Custom|OnPlayerMove
  (bind _mainwidget (Variables|Default|GetMainWidget))
  (bind _w_minimap (Variables|/Game/HUD/W_HUD.W_HUD_C|GetW_MiniMap _mainwidget))
  (bind _directionarrow (Variables|/Game/HUD/W_MiniMap.W_MiniMap_C|GetDirectionArrow _w_minimap))
  (Utilities|IsValid (Variables|Default|GetCurrentGoalActor)
    (:Is%20Valid
      (bind _output_get (Variables|Default|SetCurrentDistance (CallFunction|DistancetoGoal)))
      (Rendering|Components|TextRender|SetText (Variables|/Game/HUD/W_HUD.W_HUD_C|GetDistanceText (Variables|Default|GetMainWidget)) (Utilities|Text|ToText(Integer) _output_get false false))
      (Math|Integer|CompareInt (Variables|Default|GetCurrentDistance) (Variables|Default|GetShowDirectionArrowAmount)
        (:>
          _)
        (:==
          _)
        (:<
          (Utilities|FlowControl|DoOnce false :!label _label
            (:Completed
              (Widget|SetVisibility _directionarrow "Hidden")
              (goto _label_2 Reset)))))
      (CallFunction|UpdateDirectionArrow)
      (Utilities|FlowControl|DoOnce false :!label _label_2
        (:Completed
          (Widget|SetVisibility _directionarrow "SelfHitTestInvisible")
          (goto _label Reset))))))

(fn ConstructionScript)

(fn SelectNewQuest
  (params (Quest :type BP%20Master%20Quest%20Object%20Reference) (SubGoal :type W%20Sub%20Goals%20Object%20Reference))
  (Utilities|IsValid (Variables|Default|GetCurrentQuest)
    (:Is%20Valid
      (Widget|SetIsEnabled (Variables|/Game/HUD/W_Quests.W_Quests_C|GetQuestName (Variables|/Game/MainAssets/Blueprints/Actors/QuestActors/BP_MasterQuest.BP_MasterQuest_C|GetQuestWidget (Variables|Default|GetCurrentQuest))) false)
      (Default|SelectSubGoal (Variables|/Game/MainAssets/Blueprints/Actors/QuestActors/BP_MasterQuest.BP_MasterQuest_C|GetQuestWidget (Variables|Default|GetCurrentQuest))))
    (:Is%20Not%20Valid
      _))
  (bind _output_get (Variables|Default|SetCurrentQuest Quest))
  (Default|OnQuestSelected (Variables|/Game/MainAssets/Blueprints/Actors/QuestActors/BP_MasterQuest.BP_MasterQuest_C|GetQuestWidget _output_get) SubGoal)
  (return))

(fn AddNewQuest
  (params (QuestClass :type BP%20Master%20Quest%20Class%20Reference) (DirectlyStart :type Boolean))
  (LocalVariables|SetLocalClass QuestClass)
  (LocalVariables|SetLocalStart DirectlyStart)
  (if (and (Utilities|IsValidClass QuestClass) (not (Utilities|Array|ContainsItem (Variables|Default|GetAllQuestClasses) QuestClass)))
    (Utilities|Array|Add (Variables|Default|GetAllQuestClasses) (LocalVariables|GetLocalClass))
    (bind _returnvalue (Game|SpawnActorfromClass (LocalVariables|GetLocalClass) (Math|Transform|MakeTransform "0, 0, 0" "0, 0, 0" "1,1,1") "AlwaysSpawn" 0 0))
    (bind _output_get (LocalVariables|SetLocalQuestActor _returnvalue))
    (Utilities|Array|Add (Variables|Default|GetQuestActors) _output_get)
    (Default|SetUpStartingGoals (LocalVariables|GetLocalQuestActor))
    (bind _questwidgetref (Default|AddQuesttoList (Variables|Default|GetMainWidget) (LocalVariables|GetLocalQuestActor)))
    (bind _output_get_2 (Variables|/Game/MainAssets/Blueprints/Actors/QuestActors/BP_MasterQuest.BP_MasterQuest_C|SetQuestWidget (LocalVariables|GetLocalQuestActor) _questwidgetref))
    (Default|UpdateQuest _output_get_2)
    (if (or (LocalVariables|GetLocalStart) (<= (Utilities|Array|Length (Variables|Default|GetQuestActors)) 1))
      (CallFunction|SelectNewQuest (LocalVariables|GetLocalQuestActor) (Utilities|Array|Get(acopy) (Variables|/Game/HUD/W_Quests.W_Quests_C|GetSubGoalWidget (Variables|/Game/MainAssets/Blueprints/Actors/QuestActors/BP_MasterQuest.BP_MasterQuest_C|GetQuestWidget (LocalVariables|GetLocalQuestActor))))))
    (return true)
    (else
      (return false))))

(fn DistancetoGoal
  (bind _oarfref (Variables|Default|GetOarfRef))
  (bind _currentgoalactor (Variables|Default|GetCurrentGoalActor))
  (bind _returnvalue (Transformation|GetActorLocation _currentgoalactor))
  (bind _returnvalue_2 (Transformation|GetActorLocation _oarfref))
  (return (Math|Float|Round (/ (Math|Vector|VectorLength (- (Math|Vector|MakeVector (.x _returnvalue_2) (.y _returnvalue_2) 0.0) (Math|Vector|MakeVector (.x _returnvalue) (.y _returnvalue) 0.0))) 1e+02))))

(fn UpdateDirectionArrow
  (Class|Widget|SetRenderTransformAngle (Variables|/Game/HUD/W_MiniMap.W_MiniMap_C|GetDirectionArrow (Variables|/Game/HUD/W_HUD.W_HUD_C|GetW_MiniMap (Variables|Default|GetMainWidget))) (.Yaw (Math|Rotator|BreakRotator (Math|Rotator|FindLookatRotation (Transformation|GetActorLocation (Variables|Default|GetOarfRef)) (Transformation|GetActorLocation (Variables|Default|GetCurrentGoalActor))))))
  (return))