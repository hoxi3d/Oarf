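; Base Blueprint for buildings that can display one of several meshes from its Meshes array.
; The mesh index is looked up in GI_Building by the actor's class, and BeginPlay applies that mesh.
; NextMesh has the game instance increment the class's index using the array length, then updates only this actor's mesh.
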(event EventBeginPlay
  (bind _asgi_building (Utilities|Casting|CastToGI_Building (Game|GetGameInstance)))
  (bind _index (Default|GetMeshIndex _asgi_building (Utilities|GetClass self)))
  (Components|StaticMesh|SetStaticMesh (Variables|Default|GetMesh) (Utilities|Array|Get(acopy) (Variables|Default|GetMeshes) _index)))

(fn ConstructionScript)

(fn NextMesh
  (bind _meshes (Variables|Default|GetMeshes))
  (bind _asgi_building (Utilities|Casting|CastToGI_Building (Game|GetGameInstance)))
  (bind _newindex (Default|IncrementMeshIndex _asgi_building (Utilities|GetClass self) (Utilities|Array|Length _meshes)))
  (Components|StaticMesh|SetStaticMesh (Variables|Default|GetMesh) (Utilities|Array|Get(acopy) _meshes _newindex)))